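; Player controller that registers an Enhanced Input context, shows the cursor and drives the cached BP_CHARACTER's movement and camera rotation.
; Each move input also increments and prints a GameInstance counter, apparently as a test of global variables.
; Debug keys reload ThirdPersonMap, print the impact point under the cursor, and draw a persistent line trace from the character's arrow.
; The hit-actor cast and GameMode counter logic are left unconnected.
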(event Input|EnhancedActionEvents|EnhancedInputActionIA_MoveCustom
  (params (ActionValue :type Vector%202D%20Structure) (ElapsedSeconds :type Float%20%28double-precision%29) (TriggeredSeconds :type Float%20%28double-precision%29) (InputAction :type Input%20Action%20Object%20Reference :default "/Game/Input/InputAction/IA_MoveCustom.IA_MoveCustom"))
  (bind _as_bp_character (Variables|Default|GetAs%20BP%20CHARACTER))
  (bind _returnvalue (Pawn|GetControlRotation _as_bp_character :!class /Script/Engine.Pawn))
  (Pawn|Input|AddMovementInput _as_bp_character (Math|Vector|GetForwardVector _returnvalue) (.x ActionValue) false)
  (Pawn|Input|AddMovementInput _as_bp_character (Math|Vector|GetRightVector _returnvalue) (.y ActionValue) false)
  (bind _asgi_global_variable (Utilities|Casting|CastToGI_GlobalVariable (Game|GetGameInstance)))
  (bind _output_get (Variables|/Game/Blueprints/GI_GlobalVariable.GI_GlobalVariable_C|SetVar1 _asgi_global_variable (+ (Variables|/Game/Blueprints/GI_GlobalVariable.GI_GlobalVariable_C|GetVar1 _asgi_global_variable) 1)))
  (Development|PrintString (Utilities|String|ToString(Integer) _output_get)))

(event Input|EnhancedActionEvents|EnhancedInputActionIA_CameraRotation
  (params (ActionValue :type Vector%202D%20Structure) (ElapsedSeconds :type Float%20%28double-precision%29) (TriggeredSeconds :type Float%20%28double-precision%29) (InputAction :type Input%20Action%20Object%20Reference :default "/Game/Input/InputAction/IA_CameraRotation.IA_CameraRotation"))
  (Pawn|Input|AddControllerYawInput (Variables|Default|GetAs%20BP%20CHARACTER) (.x ActionValue))
  (Pawn|Input|AddControllerPitchInput (Variables|Default|GetAs%20BP%20CHARACTER) (.y ActionValue)))

(event EventBeginPlay
  (bind _returnvalue (PlayerController|LocalPlayerSubsystems|GetEnhancedInputLocalPlayerSubsystem))
  (Utilities|IsValid _returnvalue
    (:Is%20Valid
      (Input|AddMappingContext _returnvalue "/Game/Input/NewInputMappingContext.NewInputMappingContext" 0 "(bIgnoreAllPressedKeysUntilRelease=True,bForceImmediately=False,bNotifyUserSettings=False)")
      (bind _asbp_character (Utilities|Casting|CastToBP_CHARACTER (Game|GetPlayerCharacter 0)))
      (Variables|Default|SetAs%20BP%20CHARACTER _asbp_character)
      (Variables|Default|SetbShowMouseCursor true))))

(event EventTick
  (params (DeltaSeconds :type Float%20%28single-precision%29)))

(event Input|KeyboardEvents|DebugKeyR
  (params (Key :type Key%20Structure :default "None") (ActionValue :type Input%20Action%20Value%20Structure))
  (:Pressed
    (Game|OpenLevel(byObjectReference) "/Game/ThirdPerson/Maps/ThirdPersonMap.ThirdPersonMap")))

(event Input|MouseEvents|LeftMouseButton
  (params (Key :type Key%20Structure :default "None"))
  (:Pressed
    (Development|PrintString (Utilities|String|ToString(Vector) (.ImpactPoint (Collision|BreakHitResult (.HitResult (Game|Player|GetHitResultUnderCursorbyChannel "TraceTypeQuery1" true))))))))

(event Input|KeyboardEvents|C
  (params (Key :type Key%20Structure :default "None"))
  (bind _as_bp_character (Variables|Default|GetAs%20BP%20CHARACTER))
  (bind _arrow1 (Variables|/Game/Blueprints/BP_CHARACTER.BP_CHARACTER_C|GetArrow1 _as_bp_character))
  (bind _returnvalue (Transformation|GetWorldLocation _arrow1))
  (:Pressed
    (bind _outhit (Collision|LineTraceByChannel _returnvalue (+ _returnvalue (* (Math|Vector|GetForwardVector _arrow1) 1e+03)) "TraceTypeQuery1" false 0 "Persistent"))))

(fn ConstructionScript)