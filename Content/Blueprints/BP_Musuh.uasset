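; BP_Musuh is an enemy actor that shows a health bar widget and loses health when hit by first-person projectiles.
; On BeginPlay it passes itself as owner to its WB_HealthBarObject widget, printing a debug message if the cast fails.
; Each tick it rotates the widget component to face the player character.
; Capsule hits from BP_FirstPersonProjectile subtract a fixed amount of Health, with no death handling.
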(event OnComponentHit(Capsule)
  (params (HitComponent :type Primitive%20Component%20Object%20Reference) (OtherActor :type Actor%20Object%20Reference) (OtherComp :type Primitive%20Component%20Object%20Reference) (NormalImpulse :type Vector :default "0, 0, 0") (Hit :type Hit%20Result%20Structure%20%28by%20ref%29))
  (Utilities|Casting|CastToBP_FirstPersonProjectile OtherActor)
  (Variables|Default|SetHealth (- (Variables|Default|GetHealth) 5.0)))

(event EventBeginPlay
  (bind _aswb_health_bar_object (Utilities|Casting|CastToWB_HealthBarObject (UserInterface|GetUserWidgetObject (Variables|Default|GetWidget)))
    (:then
      (Variables|/Game/Blueprints/WB_HealthBarObject.WB_HealthBarObject_C|SetOwner _aswb_health_bar_object self))
    (:CastFailed
      (Development|PrintString "Hello"))))

(event Collision|EventActorBeginOverlap
  (params (OtherActor :type Actor%20Object%20Reference)))

(event EventTick
  (params (DeltaSeconds :type Float%20%28single-precision%29))
  (bind _widget (Variables|Default|GetWidget))
  (Transformation|SetWorldRotation _widget (Math|Rotator|FindLookatRotation (Transformation|GetWorldLocation _widget) (Transformation|GetActorLocation (Game|GetPlayerCharacter 0))) false false))

(fn ConstructionScript)