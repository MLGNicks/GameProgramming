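; BP_BasicAI is a basic turret-like enemy that turns toward a player it sees and shoots at it.
; PawnSensing stores the seen third-person character and sets Target and Shoot flags.
; Tick lerps rotation toward it, fires one impulse-driven projectile per sighting event, and drops the target beyond a distance threshold.
; BeginPlay gathers BP_Location patrol points, but patrol movement and AIMoveTo chase logic are disconnected.
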(event OnSeePawn(PawnSensing)
  (params (Pawn :type Pawn%20Object%20Reference))
  (bind _asbp_third_person_character (Utilities|Casting|CastToBP_ThirdPersonCharacter Pawn))
  (Variables|Default|SetTarget true)
  (Variables|Default|SetShoot true)
  (Variables|Default|SetBPThirdPersonCharacter _asbp_third_person_character))

(event EventBeginPlay
  ;[1 1 1] Patrol AI (Cara 2), location actor seperate spawn di world
  (bind _outactors (Actor|GetAllActorsOfClass "/Game/Blueprints/AI/BP_Location.BP_Location_C"))
  (for _array_element _outactors
    (Utilities|Array|Add (Variables|Default|GetPatrolLoc) (Transformation|GetWorldLocation (Variables|/Game/Blueprints/AI/BP_Location.BP_Location_C|GetDefaultSceneRoot _array_element)))))

(event Collision|EventActorBeginOverlap
  (params (OtherActor :type Actor%20Object%20Reference)))

(event EventTick
  (params (DeltaSeconds :type Float%20%28single-precision%29))
  ;[1 1 1] AI Look at, biar animation look at smooth pake lerp (rotation) karena ada alpha(seconds) perlu connect ke event tick
  (if (Variables|Default|GetTarget)
    (Utilities|FlowControl|Sequence
      (:then_0
        (Transformation|SetActorRotation (Math|Rotator|Lerp(Rotator) (Transformation|GetActorRotation) (Math|Rotator|FindLookatRotation (Transformation|GetActorLocation) (Transformation|GetActorLocation (Variables|Default|GetBPThirdPersonCharacter))) 0.5))
        (if (> (Math|Vector|Distance(Vector) (Transformation|GetActorLocation) (Transformation|GetActorLocation (Variables|Default|GetBPThirdPersonCharacter))) 5e+02)
          (Variables|Default|SetTarget false)
          (Variables|Default|SetShoot false)))
      (:then_1
        ;[1 1 1] AI Shoot
        (if (Variables|Default|GetShoot)
          (bind _returnvalue (Game|SpawnActorfromClass "/Game/FirstPerson/Blueprints/BP_FirstPersonProjectile.BP_FirstPersonProjectile_C" (Transformation|GetWorldTransform (Variables|Default|GetStaticMesh)) "Undefined" "MultiplyWithRoot" 0 0))
          (Physics|AddImpulse (Variables|/Game/FirstPerson/Blueprints/BP_FirstPersonProjectile.BP_FirstPersonProjectile_C|GetSphere _returnvalue) (* (Math|Vector|GetForwardVector (Variables|Default|GetCube)) (Variables|Default|GetForce)) "None" true)
          (Variables|Default|SetShoot false)
          (Utilities|FlowControl|Delay 0.2))))))

(fn ConstructionScript)

(fn GetRandomLocation
  (Variables|Default|SetTargetLocation (Math|Random|RandomInteger (Utilities|Array|Length (Variables|Default|GetPatrolLoc)))))