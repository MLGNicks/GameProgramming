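; Character Blueprint that tracks Health and serves as a simple event test bed, with no death or clamping logic.
; BeginPlay calls CallEDCallObject, which by its name fires an event dispatcher, and the Damage event subtracts incoming damage from Health.
; Actor overlaps print the other actor's display name for debugging.
; Tick, mesh overlap and the construction script are empty, and a Health print node is left unconnected.
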(event OnComponentBeginOverlap(Mesh)
  (params (OverlappedComponent :type Primitive%20Component%20Object%20Reference) (OtherActor :type Actor%20Object%20Reference) (OtherComp :type Primitive%20Component%20Object%20Reference) (OtherBodyIndex :type Integer) (bFromSweep :type Boolean) (SweepResult :type Hit%20Result%20Structure%20%28by%20ref%29)))

(event EventBeginPlay
  (Default|CallEDCallObject))

(event EventTick
  (params (DeltaSeconds :type Float%20%28single-precision%29)))

(event EventDamage
  (params (Damage :type Integer))
  (Variables|Default|SetHealth (- (Variables|Default|GetHealth) Damage)))

(event Collision|EventActorBeginOverlap
  (params (OtherActor :type Actor%20Object%20Reference))
  (Development|PrintString (Utilities|GetDisplayName OtherActor)))

(fn ConstructionScript)