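; BP_OBJECT is a cube actor with a box trigger that damages overlapping actors through the BI_Damage interface.
; On BeginPlay it binds its name printout to BP_CHARACTER's event dispatcher and spawns a BP_SPHERE at a fixed location.
; The construction script sets the cube's material.
; Health countdown, timer, spawning and timeline rotation experiments remain in the graph but are disconnected.
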(event OnComponentBeginOverlap(Box)
  (params (OverlappedComponent :type Primitive%20Component%20Object%20Reference) (OtherActor :type Actor%20Object%20Reference) (OtherComp :type Primitive%20Component%20Object%20Reference) (OtherBodyIndex :type Integer) (bFromSweep :type Boolean) (SweepResult :type Hit%20Result%20Structure%20%28by%20ref%29))
  (if (Utilities|DoesObjectImplementInterface OtherActor "/Game/Blueprints/BI_Damage.BI_Damage_C")
    (Class|BIDamage|Damage(Message) OtherActor 10)))

(event OnComponentEndOverlap(Box)
  (params (OverlappedComponent :type Primitive%20Component%20Object%20Reference) (OtherActor :type Actor%20Object%20Reference) (OtherComp :type Primitive%20Component%20Object%20Reference) (OtherBodyIndex :type Integer))
  (Development|PrintString "not overlapping"))

(event Custom|CekDarah
  ;[1 1 1] Cek HP + Event Timer
  (if (>= (Variables|Default|GetHealth) 1)
    (bind _output_get (Variables|Default|SetHealth (- (Variables|Default|GetHealth) 1)))
    (Development|PrintString (Utilities|String|ToString(Integer) _output_get))
    (else
      (Game|QuitGame 0 "Quit" false))))

(event Custom|PrintIdentity
  (Development|PrintString (Utilities|GetDisplayName self)))

(event EventBeginPlay
  (bind _asbp_character (Utilities|Casting|CastToBP_CHARACTER (Game|GetPlayerCharacter 0)))
  (EventDispatchers|BindEventtoEDCallObject _asbp_character (delegate Custom|PrintIdentity))
  (Game|SpawnActorfromClass "/Game/Blueprints/BP_SPHERE.BP_SPHERE_C" (Math|Transform|MakeTransform "1700.000000,600.000000,85.000000") "Undefined" "MultiplyWithRoot" 0 0))

(event Collision|EventActorBeginOverlap
  (params (OtherActor :type Actor%20Object%20Reference)))

(event EventTick
  (params (DeltaSeconds :type Float%20%28single-precision%29)))

(fn ConstructionScript
  (Rendering|Material|SetMaterial (Variables|Default|GetCube) 0 (Variables|Default|GetCube%20Material)))

(fn CekHP
  (if (> (Variables|Default|GetHealth) 0)
    (bind _output_get (Variables|Default|SetHealth (- (Variables|Default|GetHealth) 1)))
    (Development|PrintString (Utilities|String|ToString(Integer) _output_get))
    (else
      (Game|QuitGame 0 "Quit" false))))